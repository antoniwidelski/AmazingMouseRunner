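; BP_MouseCharacter is a touch-controlled mouse character that jumps or moves down on vertical swipes.
; A touch calls Clicked and records its start; Tick then samples Touch1 through a DoOnce, calling MJump or Down by vertical direction.
; Release resets the DoOnce but never clears IsPressed, and the swipe-length check does nothing.
; Separate events play an enemy-jump animation, set the mouse AnimBP, and show a flash widget.
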(event `self.ReceiveBeginPlay`)

(event `self.ReceiveTick`
  (params (DeltaSeconds :type "Float (single-precision)"))
  (bind (_locationx _locationy) (`PlayerController.GetInputTouchState` (`GameplayStatics.GetPlayerController` 0) "Touch1"))
  (bind (_returnvalue_x _returnvalue_y) (`KismetMathLibrary.BreakVector2D` (- (`self.TouchStart`) (`self.TouchEnd`))))
  (if (`self.IsPressed`)
    (`/Engine/EditorBlueprintResources/StandardMacros.DoOnce` false :!label _label
      (:`Completed`
        (set `self.TouchEnd` (`KismetMathLibrary.MakeVector2D` _locationx _locationy))
        (if (> (`KismetMathLibrary.Abs` _returnvalue_x) (`KismetMathLibrary.Abs` _returnvalue_y))
          _
          (elif (> _returnvalue_y 0.0)
            (`self.MJump`)
            (elif (< _returnvalue_y 0.0)
              (`self.Down`))))))))

(event `InputTouch`
  (params (Location :type "Vector Structure") (FingerIndex :type "ETouchIndex Enum"))
  (bind (_x _y) (`KismetMathLibrary.BreakVector3f` Location))
  (:`Pressed`
    (`self.Clicked`)
    (set `self.IsPressed` true)
    (set `self.TouchStart` (`KismetMathLibrary.MakeVector2D` _x _y)))
  (:`Released`
    (set `self.TouchEnd` (`KismetMathLibrary.MakeVector2D` _x _y))
    (goto _label :!via `Reset`)))

(event `Check_Swiping`
  (if (> (`KismetMathLibrary.VSize2D` (- (`self.TouchStart`) (`self.TouchEnd`))) 100.0)
    _))

(event `self.PlayEnemyJumpAnimation`
  (`SkeletalMeshComponent.PlayAnimation` (`self.Mesh`) "/Game/Mesh/Mouse/JumpEnemy.JumpEnemy" false)
  (`SkeletalMeshComponent.SetAnimInstanceClass` (`self.Mesh`) "/Game/Blueprints/PlayerRelated/ABP_Mouse.ABP_Mouse_C"))

(event `self.Flash`
  (bind _returnvalue (`|CreateWidget` "/Game/Menu/WBP_Flash.WBP_Flash_C"))
  (`UserWidget.AddToViewport` _returnvalue 0))

(fn `UserConstructionScript`)
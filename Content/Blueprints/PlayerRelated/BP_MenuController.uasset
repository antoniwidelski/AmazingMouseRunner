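; BP_MenuController switches the game between its menu screens: main, shop, fence, color and best scores.
; Each menu has its own event that removes all widgets, then creates that menu's widget and adds it to the viewport.
; Widgets are created fresh on every switch rather than cached, and nothing in this Blueprint calls the events itself.
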(event `MainMenu`
  (`WidgetLayoutLibrary.RemoveAllWidgets`)
  (bind _returnvalue (`|CreateWidget` "/Game/Menu/WBP_MainMenu.WBP_MainMenu_C"))
  (`UserWidget.AddToViewport` _returnvalue 0))

(event `ShopMenu`
  (`WidgetLayoutLibrary.RemoveAllWidgets`)
  (bind _returnvalue (`|CreateWidget` "/Game/Menu/WBP_ShopMenu.WBP_ShopMenu_C"))
  (`UserWidget.AddToViewport` _returnvalue 0))

(event `FenceMenu`
  (`WidgetLayoutLibrary.RemoveAllWidgets`)
  (bind _returnvalue (`|CreateWidget` "/Game/Menu/WBP_FenceMenu.WBP_FenceMenu_C"))
  (`UserWidget.AddToViewport` _returnvalue 0))

(event `ColorMenu`
  (`WidgetLayoutLibrary.RemoveAllWidgets`)
  (bind _returnvalue (`|CreateWidget` "/Game/Menu/WBP_ColorMenu.WBP_ColorMenu_C"))
  (`UserWidget.AddToViewport` _returnvalue 0))

(event `ScoreMenu`
  (`WidgetLayoutLibrary.RemoveAllWidgets`)
  (bind _returnvalue (`|CreateWidget` "/Game/Menu/WBP_BestScores.WBP_BestScores_C"))
  (`UserWidget.AddToViewport` _returnvalue 0))

(fn `UserConstructionScript`)
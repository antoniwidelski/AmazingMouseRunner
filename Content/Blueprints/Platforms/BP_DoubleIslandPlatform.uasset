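; BP_DoubleIslandPlatform is a platform Blueprint whose meshes take their material from the game's current color type.
; Its construction script reads the color type from BP_MouseGameInstance and looks up the matching platform material by index.
; It creates one dynamic material instance from that material and shares it across slot 0 of all four static meshes.
; The event graph contains no gameplay logic.
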(event `self.ReceiveBeginPlay`)

(fn `UserConstructionScript`
  (bind _asbp_mouse_game_instance (cast `/Game/Blueprints/Other/BP_MouseGameInstance` (`GameplayStatics.GetGameInstance`)))
  (bind _returnvalue (`KismetMaterialLibrary.CreateDynamicMaterialInstance` (`self.GetPlatformMaterialByIndex` (`MouseGameInstance.GetColorType` _asbp_mouse_game_instance))))
  (bind _output_get (set `self.NewMaterial` _returnvalue))
  (`PrimitiveComponent.SetMaterial` (`self.StaticMesh`) 0 _output_get)
  (`PrimitiveComponent.SetMaterial` (`self.StaticMesh2`) 0 _output_get)
  (`PrimitiveComponent.SetMaterial` (`self.StaticMesh1`) 0 _output_get)
  (`PrimitiveComponent.SetMaterial` (`self.Mesh`) 0 _output_get))
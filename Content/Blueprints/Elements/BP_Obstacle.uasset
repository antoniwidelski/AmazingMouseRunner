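; BP_Obstacle is an obstacle actor whose mesh matches the fence type held by the game instance.
; On BeginPlay it casts the game instance to BP_MouseGameInstance, reads GetFenceType and sets its Mesh to a fence, stone wall or metal fence.
; Unrecognized types fall back to the fence mesh, and a failed cast leaves the mesh unchanged.
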(event `self.ReceiveBeginPlay`
  (bind _asbp_mouse_game_instance (cast `/Game/Blueprints/Other/BP_MouseGameInstance` (`GameplayStatics.GetGameInstance`)))
  (switch `int` (`MouseGameInstance.GetFenceType` _asbp_mouse_game_instance)
    (:`Default`
      (`StaticMeshComponent.SetStaticMesh` (`self.Mesh`) "/Game/Mesh/Fence/Fence.Fence"))
    (:`0`
      (`StaticMeshComponent.SetStaticMesh` (`self.Mesh`) "/Game/Mesh/Fence/Fence.Fence"))
    (:`1`
      (`StaticMeshComponent.SetStaticMesh` (`self.Mesh`) "/Game/Mesh/Stonewall/stonewall.stonewall"))
    (:`2`
      (`StaticMeshComponent.SetStaticMesh` (`self.Mesh`) "/Game/Mesh/MetalFence/metalfence.metalfence"))))

(fn `UserConstructionScript`)